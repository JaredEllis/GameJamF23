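; Modular boxwood bush that acts as a hiding spot for the player.
; The construction script calls ConstructBush, which sets the static mesh from the Type enum and a uniform scale from the Size enum.
; A Randomize function picks both enums at random and rebuilds the bush.
; Box overlap events set IsHidden on BP_Player when it enters and clear it when it leaves.
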(event OnComponentBeginOverlap(Box)
  (params (OverlappedComponent :type Primitive%20Component%20Object%20Reference) (OtherActor :type Actor%20Object%20Reference) (OtherComp :type Primitive%20Component%20Object%20Reference) (OtherBodyIndex :type Integer) (bFromSweep :type Boolean) (SweepResult :type Hit%20Result%20Structure%20%28by%20ref%29))
  (bind _actor (Utilities|IsObjectClass? OtherActor "/Game/Systems/Player/BP_Player.BP_Player_C")
    (:IsClass
      (bind _asbp_player (Utilities|Casting|CastToBP_Player _actor))
      (Variables|/Game/Systems/Player/BP_Player.BP_Player_C|SetisHidden _asbp_player true))))

(event OnComponentEndOverlap(Box)
  (params (OverlappedComponent :type Primitive%20Component%20Object%20Reference) (OtherActor :type Actor%20Object%20Reference) (OtherComp :type Primitive%20Component%20Object%20Reference) (OtherBodyIndex :type Integer))
  (bind _actor (Utilities|IsObjectClass? OtherActor "/Game/Systems/Player/BP_Player.BP_Player_C")
    (:IsClass
      (bind _asbp_player (Utilities|Casting|CastToBP_Player _actor))
      (Variables|/Game/Systems/Player/BP_Player.BP_Player_C|SetisHidden _asbp_player false))))

(fn ConstructionScript
  (CallFunction|ConstructBush))

(fn Randomize
  (Variables|Default|SetType (Utilities|Enum|ByteToEnumE_BushType (Math|Conversions|ToByte(Integer) (Math|Random|RandomInteger (|GetNumEnumEntries)))))
  (Variables|Default|SetSize (Utilities|Enum|ByteToEnumE_BushSizes (Math|Conversions|ToByte(Integer) (Math|Random|RandomInteger (|GetNumEnumEntries)))))
  (CallFunction|ConstructBush))

(fn ConstructBush
  (Components|StaticMesh|SetStaticMesh (Variables|Default|GetStaticMesh) (Utilities|Select :Index (Variables|Default|GetType) :NewEnumerator0 "/Game/Megascans/3D_Plants/Boxwood_wfypfa3ha/S_Boxwood_wfypfa3ha_Var7_lod3.S_Boxwood_wfypfa3ha_Var7_lod3" :NewEnumerator3 "/Game/Megascans/3D_Plants/Boxwood_wfypfa3ha/S_Boxwood_wfypfa3ha_Var6_lod3.S_Boxwood_wfypfa3ha_Var6_lod3" :NewEnumerator1 "/Game/Megascans/3D_Plants/Boxwood_wfypfa3ha/S_Boxwood_wfypfa3ha_Var9_lod3.S_Boxwood_wfypfa3ha_Var9_lod3"))
  (Transformation|SetRelativeScale3D (Variables|Default|GetStaticMesh) (Utilities|Select :Index (Variables|Default|GetSize) :NewEnumerator0 "1.000000,1.000000,1.000000" :NewEnumerator1 "2.000000,2.000000,2.000000" :NewEnumerator2 "3.000000,3.000000,3.000000")))
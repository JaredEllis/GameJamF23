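; Base door actor with an animated skeletal mesh that blocks until opened and shows a HUD tip to a nearby player.
; OpenDoor runs once, plays the cell-door animation, then after a fixed delay disables collision and calls OnDoorOpen.
; Box overlap shows the tip only if the player has a key and clears it on exit; it never opens the door itself.
; The construction script applies the configurable mesh.
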(event OnComponentBeginOverlap(Box)
  (params (OverlappedComponent :type Primitive%20Component%20Object%20Reference) (OtherActor :type Actor%20Object%20Reference) (OtherComp :type Primitive%20Component%20Object%20Reference) (OtherBodyIndex :type Integer) (bFromSweep :type Boolean) (SweepResult :type Hit%20Result%20Structure%20%28by%20ref%29))
  (Utilities|IsObjectClass? OtherActor "/Game/Systems/Player/BP_Player.BP_Player_C"
    (:IsClass
      (bind _player (Class|BPIGameMode|FreePlayerCast(Message) (Game|GetGameMode)))
      (if (Variables|/Game/Systems/Player/BP_Player.BP_Player_C|GethasKey _player)
        (Default|ShowTextTip (Variables|/Game/Systems/Player/BP_Player.BP_Player_C|GetHUD _player) (Variables|Default|GetText))
        (Development|PrintString "Hello")))))

(event OnComponentEndOverlap(Box)
  (params (OverlappedComponent :type Primitive%20Component%20Object%20Reference) (OtherActor :type Actor%20Object%20Reference) (OtherComp :type Primitive%20Component%20Object%20Reference) (OtherBodyIndex :type Integer))
  (Utilities|IsObjectClass? OtherActor "/Game/Systems/Player/BP_Player.BP_Player_C"
    (:IsClass
      (bind _player (Class|BPIGameMode|FreePlayerCast(Message) (Game|GetGameMode)))
      (Default|ShowTextTip (Variables|/Game/Systems/Player/BP_Player.BP_Player_C|GetHUD _player)))))

(event Custom|OpenDoor
  (Utilities|FlowControl|DoOnce false
    (:Completed
      (Components|Animation|PlayAnimation (Variables|Default|GetSkeletalMesh) "/Game/Art/Environment/Meshes/Cell-Door/SM_cellDoor_Anim_Anim.SM_cellDoor_Anim_Anim" false)
      (Utilities|FlowControl|Delay 2.0)
      (Collision|SetCollisionEnabled (Variables|Default|GetSkeletalMesh) "NoCollision")
      (Default|CallOnDoorOpen))))

(event EventBeginPlay
  (Collision|SetCollisionEnabled (Variables|Default|GetSkeletalMesh) "QueryAndPhysics"))

(fn ConstructionScript
  (Components|SkeletalMesh|SetSkeletalMeshAsset (Variables|Default|GetSkeletalMesh) (Variables|Default|GetNew%20SK)))
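; BP_TextTip is a trigger volume that shows a text tip on the HUD while BP_Player is inside it.
; On begin overlap it passes its Text to ShowTextTip on the HUD, reached through the game mode's FreePlayerCastMessage.
; On end overlap it waits briefly, then clears the tip with an empty string.
; The construction script sizes the Trigger box from the InBoxExtent variable.
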(event OnComponentBeginOverlap(Trigger)
  (params (OverlappedComponent :type Primitive%20Component%20Object%20Reference) (OtherActor :type Actor%20Object%20Reference) (OtherComp :type Primitive%20Component%20Object%20Reference) (OtherBodyIndex :type Integer) (bFromSweep :type Boolean) (SweepResult :type Hit%20Result%20Structure%20%28by%20ref%29))
  (Utilities|IsObjectClass? OtherActor "/Game/Systems/Player/BP_Player.BP_Player_C"
    (:IsClass
      (bind _player (Class|BPIGameMode|FreePlayerCast(Message) (Game|GetGameMode)))
      (Default|ShowTextTip (Variables|/Game/Systems/Player/BP_Player.BP_Player_C|GetHUD _player) (Variables|Default|GetText)))))

(event OnComponentEndOverlap(Trigger)
  (params (OverlappedComponent :type Primitive%20Component%20Object%20Reference) (OtherActor :type Actor%20Object%20Reference) (OtherComp :type Primitive%20Component%20Object%20Reference) (OtherBodyIndex :type Integer))
  (Utilities|IsObjectClass? OtherActor "/Game/Systems/Player/BP_Player.BP_Player_C"
    (:IsClass
      (bind _player (Class|BPIGameMode|FreePlayerCast(Message) (Game|GetGameMode)))
      (Utilities|FlowControl|Delay 2.0)
      (Default|ShowTextTip (Variables|/Game/Systems/Player/BP_Player.BP_Player_C|GetHUD _player)))))

(fn ConstructionScript
  (Components|Box|SetBoxExtent (Variables|Default|GetTrigger) (Variables|Default|GetIn%20Box%20Extent) true))
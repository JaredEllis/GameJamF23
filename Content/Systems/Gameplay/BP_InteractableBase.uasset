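; BP_InteractableBase is an interactable actor that shows a text prompt on the player's HUD.
; The construction script applies its mesh, scale and sphere radius, and BeginPlay initializes the WBP_Interact widget's text and size.
; Tick shows the tip when the player is near and roughly facing the mesh, comparing absolute yaws, and otherwise clears it every frame.
; Sphere overlap events are empty, leaving older overlap-style tip logic disconnected.
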(event OnComponentBeginOverlap(Sphere)
  (params (OverlappedComponent :type Primitive%20Component%20Object%20Reference) (OtherActor :type Actor%20Object%20Reference) (OtherComp :type Primitive%20Component%20Object%20Reference) (OtherBodyIndex :type Integer) (bFromSweep :type Boolean) (SweepResult :type Hit%20Result%20Structure%20%28by%20ref%29)))

(event OnComponentEndOverlap(Sphere)
  (params (OverlappedComponent :type Primitive%20Component%20Object%20Reference) (OtherActor :type Actor%20Object%20Reference) (OtherComp :type Primitive%20Component%20Object%20Reference) (OtherBodyIndex :type Integer)))

(event EventBeginPlay
  (bind _aswbp_interact (Utilities|Casting|CastToWBP_Interact (UserInterface|GetUserWidgetObject (Variables|Default|GetWidget1))))
  (Default|InitTextandFont _aswbp_interact (Variables|Default|GetString) (Variables|Default|GetSize)))

(event EventTick
  (params (DeltaSeconds :type Float%20%28single-precision%29))
  (bind _staticmesh (Variables|Default|GetStaticMesh))
  (bind _returnvalue (Transformation|GetWorldLocation _staticmesh))
  (bind _player (Class|BPIGameMode|FreePlayerCast(Message) (Game|GetGameMode)))
  (if (and (Math|Float|InRange(Float) (Math|Float|Absolute(Float) (.Yaw (Math|Rotator|BreakRotator (Transformation|GetActorRotation _player)))) (- (Math|Float|Absolute(Float) (.Yaw (Math|Rotator|BreakRotator (Math|Rotator|FindLookatRotation (Transformation|GetActorLocation _player) _returnvalue)))) 15.0) (+ (Math|Float|Absolute(Float) (.Yaw (Math|Rotator|BreakRotator (Math|Rotator|FindLookatRotation (Transformation|GetActorLocation _player) _returnvalue)))) 15.0)) (< (Math|Vector|Distance(Vector) (Transformation|GetActorLocation _player) _returnvalue) 2e+02))
    (Default|ShowTextTip (Variables|/Game/Systems/Player/BP_Player.BP_Player_C|GetHUD _player) (Variables|Default|GetString))
    (else
      (Default|ShowTextTip (Variables|/Game/Systems/Player/BP_Player.BP_Player_C|GetHUD _player)))))

(fn ConstructionScript
  (Components|StaticMesh|SetStaticMesh (Variables|Default|GetStaticMesh) (Variables|Default|GetNew%20Mesh))
  (Transformation|SetRelativeScale3D (Variables|Default|GetStaticMesh) (Variables|Default|GetNew%20Scale%203D))
  (Components|Sphere|SetSphereRadius (Variables|Default|GetSphere) (Variables|Default|GetIn%20Sphere%20Radius) true))
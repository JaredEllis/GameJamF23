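; BP_SleepingGuard is a guard enemy that shows the player a text tip when they are close and facing it.
; Each Tick, once the player's OpenedDoor is true, it compares absolute player yaw to the look-at yaw within a narrow tolerance, checks distance, then sets or clears the HUD tip.
; The box overlap event is empty, and the "Press E to Bite" prompt and Takedown call are unwired.
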(event OnComponentBeginOverlap(Box)
  (params (OverlappedComponent :type Primitive%20Component%20Object%20Reference) (OtherActor :type Actor%20Object%20Reference) (OtherComp :type Primitive%20Component%20Object%20Reference) (OtherBodyIndex :type Integer) (bFromSweep :type Boolean) (SweepResult :type Hit%20Result%20Structure%20%28by%20ref%29)))

(event EventTick
  (params (DeltaSeconds :type Float%20%28single-precision%29))
  (bind _staticmesh (Variables|Default|GetStaticMesh))
  (bind _returnvalue (Transformation|GetWorldLocation _staticmesh))
  (bind _player (Class|BPIGameMode|FreePlayerCast(Message) (Game|GetGameMode)))
  (if (Variables|/Game/Systems/Player/BP_Player.BP_Player_C|GetopenedDoor _player)
    (if (and (Math|Float|InRange(Float) (Math|Float|Absolute(Float) (.Yaw (Math|Rotator|BreakRotator (Transformation|GetActorRotation _player)))) (- (Math|Float|Absolute(Float) (.Yaw (Math|Rotator|BreakRotator (Math|Rotator|FindLookatRotation (Transformation|GetActorLocation _player) _returnvalue)))) 15.0) (+ (Math|Float|Absolute(Float) (.Yaw (Math|Rotator|BreakRotator (Math|Rotator|FindLookatRotation (Transformation|GetActorLocation _player) _returnvalue)))) 15.0)) (< (Math|Vector|Distance(Vector) (Transformation|GetActorLocation _player) _returnvalue) 2e+02))
      (Default|ShowTextTip (Variables|/Game/Systems/Player/BP_Player.BP_Player_C|GetHUD _player) (Variables|Default|GetString))
      (else
        (Default|ShowTextTip (Variables|/Game/Systems/Player/BP_Player.BP_Player_C|GetHUD _player))))))

(fn ConstructionScript)
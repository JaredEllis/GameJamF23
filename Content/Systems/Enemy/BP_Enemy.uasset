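; BP_Enemy is an enemy actor with an alert state and a takedown that the player can be granted.
; SetAlerted stores the state and prints it through a DoOnce, which RestartAlert resets.
; Overlapping TakedownArea, a box sized in the construction script, toggles CanTakedown on BP_Player.
; TakeDown disables movement and collision, calls PlayAnimMontage, then destroys the actor after the returned duration.
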(event OnComponentBeginOverlap(TakedownArea)
  (params (OverlappedComponent :type Primitive%20Component%20Object%20Reference) (OtherActor :type Actor%20Object%20Reference) (OtherComp :type Primitive%20Component%20Object%20Reference) (OtherBodyIndex :type Integer) (bFromSweep :type Boolean) (SweepResult :type Hit%20Result%20Structure%20%28by%20ref%29))
  (bind _asbp_player (Utilities|Casting|CastToBP_Player OtherActor))
  (Variables|/Game/Systems/Player/BP_Player.BP_Player_C|SetcanTakedown _asbp_player true))

(event OnComponentEndOverlap(TakedownArea)
  (params (OverlappedComponent :type Primitive%20Component%20Object%20Reference) (OtherActor :type Actor%20Object%20Reference) (OtherComp :type Primitive%20Component%20Object%20Reference) (OtherBodyIndex :type Integer))
  (bind _asbp_player (Utilities|Casting|CastToBP_Player OtherActor))
  (Variables|/Game/Systems/Player/BP_Player.BP_Player_C|SetcanTakedown _asbp_player false))

(event Custom|RestartAlert
  (Utilities|FlowControl|DoOnce false) ; enters at Reset
)

(event Custom|TakeDown
  (Pawn|Components|CharacterMovement|DisableMovement (Variables|Character|GetCharacterMovement))
  (Collision|SetActorEnableCollision false)
  (bind _returnvalue (Animation|PlayAnimMontage 0 1.0 "None"))
  (Utilities|FlowControl|Delay _returnvalue)
  (Actor|DestroyActor))

(event EventSetAlerted
  (params (AlertState :type E_AlertState%20Enum :default "NewEnumerator0"))
  (Variables|Default|SetAlertState AlertState)
  (Utilities|FlowControl|DoOnce false
    (:Completed
      (Development|PrintString (Utilities|String|EnumtoString (Variables|Default|GetAlertState))))))

(fn ConstructionScript
  (Components|Box|SetBoxExtent (Variables|Default|GetTakedownArea) (Variables|Default|GetIn%20Box%20Extent) true))